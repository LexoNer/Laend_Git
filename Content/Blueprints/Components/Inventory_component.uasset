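; Inventory component that tracks item quantities in a map keyed by item ID, with hoe and watering can references passed through on adding.
; Adding stacks the quantity, while removing decrements by one and deletes the entry at zero.
; Both functions then update the player character's MenuSlot UI.
; The add loop returns after its first pass, so the menu receives a single one-unit update per call.
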(event EventBeginPlay)

(event EventTick
  (params (DeltaSeconds :type Float%20%28single-precision%29)))

(fn RemovefromInventory
  (params (Item_ID :type Integer))
  (bind _inventorymap (Variables|Default|GetInventoryMap))
  (bind _inventorymap_2 (Variables|Default|GetInventoryMap))
  (bind (_value _returnvalue) (Utilities|Map|Find _inventorymap Item_ID))
  (bind _returnvalue_2 (- _value 1))
  (if _returnvalue
    (if (<= _returnvalue_2 0)
      (Utilities|Map|Remove _inventorymap_2 Item_ID)
      (else
        (Utilities|Map|Add _inventorymap_2 Item_ID _returnvalue_2)))
    (bind _asplayer_character (Utilities|Casting|CastToPlayer_Character (Game|GetPlayerCharacter 0)))
    (Default|UpdateInventory (Variables|/Game/Blueprints/Characters/Player_Character/Player_Character.Player_Character_C|GetMenuSlot _asplayer_character) Item_ID 0 false)))

(fn AddtoInventory
  (params (ID_Item :type Integer) (Quantly :type Integer) (ActorObj :type Actor%20Object%20Reference) (Hoe :type Hoe%20Object%20Reference) (WateringCan :type Watering%20Can%20Object%20Reference))
  (bind _inventorymap (Variables|Default|GetInventoryMap))
  (bind (_value _returnvalue) (Utilities|Map|Find _inventorymap ID_Item))
  (if _returnvalue
    (Utilities|Map|Add (Variables|Default|GetInventoryMap) ID_Item (+ Quantly _value))
    (else
      (Utilities|Map|Add (Variables|Default|GetInventoryMap) ID_Item Quantly)))
  (bind _asplayer_character (Utilities|Casting|CastToPlayer_Character (Game|GetPlayerCharacter 0)))
  (for _index (range 0 Quantly)
    (Default|UpdateInventory (Variables|/Game/Blueprints/Characters/Player_Character/Player_Character.Player_Character_C|GetMenuSlot _asplayer_character) ID_Item 1 true ActorObj Hoe WateringCan)
    (return)))