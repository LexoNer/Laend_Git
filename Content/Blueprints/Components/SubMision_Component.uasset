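; Quest-tracking component, read from Player_Character, that runs main missions made of sequential, typed sub-missions.
; BeginPlay caches mission rows from a DataTable; AcceptMision loads type-specific data for elimination, talk and search steps, spawning search items.
; Eliminacion counts matching kills and Busqueda removes collected items, both calling CompletarMision to auto-accept the next step or quest.
; Other types are print-only or empty; Hablar and AccionesEnMision are unimplemented.
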(event EventBeginPlay
  (for _index (range 1 10)
    (bind _returnvalue (Utilities|GetDataTableRow "/Game/Blueprints/DataTables/DataTable_Submision/SubMision_DataTable.SubMision_DataTable" (Utilities|String|StringToName (Utilities|String|ToString(Integer) _index)))
      (:then
        (Utilities|Array|Add (Variables|Default|GetMisiones) _returnvalue)))))

(event EventTick
  (params (DeltaSeconds :type Float%20%28single-precision%29)))

(fn AcceptMision
  (Variables|Default|SetMisionAceptada true)
  (bind (_array_element _array_index) (Utilities|Array|ForEachLoopwithBreak (Variables|Default|GetMisiones) :!label _label)
    (:LoopBody
      (if (== _array_index (Variables|Default|GetNumeroDeMision))
        (bind _output_get (Variables|Default|SetMainQuest _array_element))
        (for (_array_element_2 _array_index_2) (.type_mision _output_get)
          (if (== _array_index_2 (Variables|Default|GetNumeroDeSubMision))
            (switch Utilities|FlowControl|Switch|SwitchonType_Mision _array_element_2
              (:NewEnumerator2
                (Development|PrintString "Llegada"))
              (:NewEnumerator0
                (Development|PrintString "Entrega"))
              (:NewEnumerator1
                (Development|PrintString "Escolta"))
              (:NewEnumerator4
                (bind _returnvalue (Utilities|GetDataTableRow "/Game/Blueprints/DataTables/DataTable_Submision/SubMisionEliminacion_DataTable.SubMisionEliminacion_DataTable" (Utilities|String|StringToName (Utilities|String|ToString(Integer) (.numberofmision _output_get))))
                  (:then
                    (Variables|Default|SetQuest_Eliminacion _returnvalue)
                    (goto _label Break))))
              (:NewEnumerator3
                (bind _returnvalue_2 (Utilities|GetDataTableRow "/Game/Blueprints/DataTables/DataTable_Mision/Mision_Hablar_DataTable.Mision_Hablar_DataTable" (Utilities|String|StringToName (Utilities|String|ToString(Integer) (.numberofmision _output_get))))
                  (:then
                    (Variables|Default|SetQuest_Hablar _returnvalue_2)
                    (goto _label Break))))
              (:NewEnumerator5
                (Development|PrintString "Lock N key"))
              (:NewEnumerator6
                (Development|PrintString "Metroidavania"))
              (:NewEnumerator7
                (Development|PrintString "Logica"))
              (:NewEnumerator8
                (Development|PrintString "Busqueda")
                (bind _returnvalue_3 (Utilities|GetDataTableRow "/Game/Blueprints/DataTables/DataTable_Mision/MisionBusqueda_DataTable.MisionBusqueda_DataTable" (Utilities|String|StringToName (Utilities|String|ToString(Integer) (.numberofmision _output_get))))
                  (:then
                    (bind _output_get_2 (Variables|Default|SetQuest_Busqueda _returnvalue_3))
                    (for (_array_element_3 _array_index_3) (.ObjetoEnInventario (Utilities|Struct|BreakMision_Busqueda_Structure _output_get_2))
                      (for (_array_element_4 _array_index_4) (.Location (Utilities|Struct|BreakMision_Busqueda_Structure _output_get_2))
                        (if (== _array_index_4 _array_index_3)
                          (Game|SpawnActorfromClass _array_element_3 (Math|Transform|MakeTransform _array_element_4 "0, 0, 0" "1,1,1") "Undefined" 0 0)
                          (goto _label Break)))))))
              (:NewEnumerator9
                (Development|PrintString "Ninguna")))))))))

(fn AccionesEnMision
  (params (type_Mision :type Type_Mision%20Enum :default "NewEnumerator0") (Kill :type Actor%20Class%20Reference)))

(fn CompletarMision
  (bind _array_index (Utilities|Array|ForEachLoopwithBreak (.type_mision (Variables|Default|GetMainQuest)) :!label _label)
    (:LoopBody
      (if (== _array_index (Variables|Default|GetNumeroDeSubMision))
        (if (== (- (Utilities|Array|Length (.type_mision (Variables|Default|GetMainQuest))) 1) (Variables|Default|GetNumeroDeSubMision))
          (Variables|Default|SetMainQuest "")
          (Variables|Default|SetQuest_Busqueda "")
          (Variables|Default|SetQuest_Eliminacion "")
          (Variables|Default|SetNumeroDeMision (+ (Variables|Default|GetNumeroDeMision) 1))
          (Variables|Default|SetNumeroDeSubMision 0)
          (Variables|Default|SetMisionAceptada false)
          (Development|PrintString "Siguiente Main Quest")
          (CallFunction|AcceptMision)
          (goto _label Break)
          (else
            (Variables|Default|SetNumeroDeSubMision (+ (Variables|Default|GetNumeroDeSubMision) 1))
            (CallFunction|AcceptMision)
            (Development|PrintString "Siguiente SubMision")
            (goto _label Break)))))))

(fn Eliminacion
  (params (Kill :type Actor%20Class%20Reference))
  (bind _quest_eliminacion (Variables|Default|GetQuest_Eliminacion))
  (bind _asplayer_character (Utilities|Casting|CastToPlayer_Character (Game|GetPlayerCharacter 0)))
  (if (== (Variables|SubMision_Component_C|GetNumeroDeMision (Variables|/Game/Blueprints/Characters/Player_Character/Player_Character.Player_Character_C|GetSubMision_Component _asplayer_character)) (.nummision _quest_eliminacion))
    (bind (_array_element _array_index) (Utilities|Array|ForEachLoopwithBreak (.submision _quest_eliminacion) :!label _label)
      (:LoopBody
        (if (== _array_element (Variables|SubMision_Component_C|GetNumeroDeSubMision (Variables|/Game/Blueprints/Characters/Player_Character/Player_Character.Player_Character_C|GetSubMision_Component _asplayer_character)))
          (bind (_array_element_2 _array_index_2) (Utilities|Array|ForEachLoopwithBreak (.referenciadelobj _quest_eliminacion) :!label _label_2)
            (:LoopBody
              (if (== _array_index_2 _array_index)
                (if (== _array_element_2 Kill)
                  (bind _output_get (Variables|Default|SetNumeroDeEliminacion (+ (Variables|Default|GetNumeroDeEliminacion) 1)))
                  (bind (_array_element_3 _array_index_3) (Utilities|Array|ForEachLoopwithBreak (.cantidad _quest_eliminacion) :!label _label_3)
                    (:LoopBody
                      (if (== _array_index_3 _array_index)
                        (if (== _array_element_3 _output_get)
                          (Variables|Default|SetNumeroDeEliminacion 0)
                          (CallFunction|CompletarMision)
                          (else
                            (goto _label_3 Break)))))
                    (:Completed
                      (goto _label_2 Break))))))
            (:Completed
              (goto _label Break))))))))

(fn Busqueda
  (params (Objeto_Recogido :type Actor%20Class%20Reference))
  (bind _quest_busqueda (Variables|Default|GetQuest_Busqueda))
  (if true
    (for _array_element (.objetoeninventario (Variables|Default|GetQuest_Busqueda))
      (if (== _array_element Objeto_Recogido)
        (Utilities|Array|RemoveItem (.objetoeninventario _quest_busqueda) Objeto_Recogido)
        (if (== 0 (Utilities|Array|Length (.objetoeninventario _quest_busqueda)))
          (CallFunction|CompletarMision))))))

(fn Hablar)