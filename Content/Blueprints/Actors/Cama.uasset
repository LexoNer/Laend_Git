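; Bed actor (Cama) that lets the player advance to a new day.
; Overlap on component R toggles the actor's input for the Player_Character, so Interact works only nearby.
; Interact calls CallSetVariables on ThirdPersonGameMode, shows the night-to-day widget (TransNoche_Dia) briefly, then increments and prints TotalDeDias.
; A DoOnce, reset after the transition, blocks repeat presses during the sequence.
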(event OnComponentBeginOverlap(r)
  (params (OverlappedComponent :type Primitive%20Component%20Object%20Reference) (OtherActor :type Actor%20Object%20Reference) (OtherComp :type Primitive%20Component%20Object%20Reference) (OtherBodyIndex :type Integer) (bFromSweep :type Boolean) (SweepResult :type Hit%20Result%20Structure%20%28by%20ref%29))
  (Utilities|Casting|CastToPlayer_Character OtherActor)
  (Input|EnableInput (Game|GetPlayerController 0)))

(event OnComponentEndOverlap(r)
  (params (OverlappedComponent :type Primitive%20Component%20Object%20Reference) (OtherActor :type Actor%20Object%20Reference) (OtherComp :type Primitive%20Component%20Object%20Reference) (OtherBodyIndex :type Integer))
  (Utilities|Casting|CastToPlayer_Character OtherActor)
  (Input|DisableInput (Game|GetPlayerController 0)))

(event EventBeginPlay)

(event Collision|EventActorBeginOverlap
  (params (OtherActor :type Actor%20Object%20Reference)))

(event EventTick
  (params (DeltaSeconds :type Float%20%28single-precision%29)))

(event Input|ActionEvents|InputActionInteract
  (params (Key :type Key%20Structure))
  (:Pressed
    (bind _asthird_person_game_mode (Utilities|Casting|CastToThirdPersonGameMode (Game|GetGameMode)))
    (Utilities|FlowControl|DoOnce false :!label _label
      (:Completed
        (Default|CallSetVariables _asthird_person_game_mode)
        (bind _returnvalue (UserInterface|CreateWidget "/Game/Blueprints/Widgets/TransNoche_Dia.TransNoche_Dia_C"))
        (UserInterface|Viewport|AddtoViewport _returnvalue 0)
        (Utilities|FlowControl|Delay 2.0)
        (Widget|RemovefromParent _returnvalue)
        (bind _result (Math|Integer|IncrementInt (Variables|Default|GetTotalDeDias))
          (:%20%20
            (Development|PrintString (Utilities|String|ToString(Integer) _result))
            (goto _label Reset)))))))

(fn ConstructionScript)