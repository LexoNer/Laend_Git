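; GridSetup is an actor that builds a grid of GridBase tiles when play begins.
; A nested loop over GridX and GridY spawns each tile at GridSize spacing, offset to roughly center the grid on the actor's location.
; Each tile receives the setup's CalidadDeTerreno (terrain quality) value and is stored in GridBaseArray.
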(event EventBeginPlay
  (bind _grid_x (Variables|Default|GetGrid_X))
  (bind _grid_y (Variables|Default|GetGrid_Y))
  (bind _gridsize (Variables|Default|GetGridSize))
  (bind _gridsize_2 (Variables|Default|GetGridSize))
  (for _index (range 1 _grid_x)
    (for _index_2 (range 1 _grid_y)
      (bind _returnvalue (Game|SpawnActorfromClass "/Game/Blueprints/Actors/GridBase.GridBase_C" (Math|Transform|MakeTransform (+ (Math|Vector|MakeVector (Math|Conversions|ToFloat(Integer) (- (* _index _gridsize_2) (/ (* _grid_x _gridsize) 2))) (Math|Conversions|ToFloat(Integer) (- (* _gridsize_2 _index_2) (/ (* _grid_y _gridsize) 2))) 0.0) (Transformation|GetActorLocation))) "AlwaysSpawn" 0 0))
      (Variables|/Game/Blueprints/Actors/GridBase.GridBase_C|SetCalidad_De_Terreno _returnvalue (Variables|Default|GetCalidad_De_Terreno))
      (Utilities|Array|Add (Variables|Default|GetGridBaseArray) _returnvalue))))

(event Collision|EventActorBeginOverlap
  (params (OtherActor :type Actor%20Object%20Reference)))

(event EventTick
  (params (DeltaSeconds :type Float%20%28single-precision%29)))

(fn ConstructionScript)