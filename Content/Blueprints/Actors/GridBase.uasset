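; Farm plot actor that the player tills, sows and waters.
; Its trigger reveals the tile and enables Interact, which tills, waters planted soil or spawns a data-table plant by held item, updating inventory and missions.
; A GameMode-bound event clears watering, while helper functions reset the plot, plant directly or raise care quality.
; Tick derives visibility and soil material from state flags, creating a new dynamic material instance every frame.
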(event OnComponentBeginOverlap(Trigger)
  (params (OverlappedComponent :type Primitive%20Component%20Object%20Reference) (OtherActor :type Actor%20Object%20Reference) (OtherComp :type Primitive%20Component%20Object%20Reference) (OtherBodyIndex :type Integer) (bFromSweep :type Boolean) (SweepResult :type Hit%20Result%20Structure%20%28by%20ref%29))
  (Utilities|Casting|CastToPlayer_Character OtherActor)
  (Rendering|SetVisibility (Variables|Default|GetGrid) true false)
  (Input|EnableInput (Game|GetPlayerController 0)))

(event OnComponentEndOverlap(Trigger)
  (params (OverlappedComponent :type Primitive%20Component%20Object%20Reference) (OtherActor :type Actor%20Object%20Reference) (OtherComp :type Primitive%20Component%20Object%20Reference) (OtherBodyIndex :type Integer))
  (Utilities|Casting|CastToPlayer_Character OtherActor)
  (if (or (Variables|Default|GetIsRake) (Variables|Default|GetPlanting?))
    (Rendering|SetVisibility (Variables|Default|GetGrid) true false)
    (Input|DisableInput (Game|GetPlayerController 0))
    (else
      (Rendering|SetVisibility (Variables|Default|GetGrid) false false)
      (Input|DisableInput 0))))

(event Custom|Prueba
  (Variables|Default|SetIsWatering? false)
  (Utilities|FlowControl|Delay 2.0))

(event EventBeginPlay
  (Rendering|SetVisibility (Variables|Default|GetGrid) false false)
  (bind _asthird_person_game_mode (Utilities|Casting|CastToThirdPersonGameMode (Game|GetGameMode)))
  (EventDispatchers|BindEventtoSetVariables _asthird_person_game_mode (delegate Custom|Prueba))
  (if (Variables|Default|GetIsWatering?)
    (Rendering|Material|CreateDynamicMaterialInstance (Variables|Default|GetGrid) 0 "/Game/Material/Tierra_Mojada.Tierra_Mojada" "None" :!class /Script/Engine.PrimitiveComponent)
    (else
      (Rendering|Material|CreateDynamicMaterialInstance (Variables|Default|GetGrid) 0 "/Game/Material/Tierra.Tierra" "None" :!class /Script/Engine.PrimitiveComponent))))

(event Collision|EventActorBeginOverlap
  (params (OtherActor :type Actor%20Object%20Reference)))

(event EventTick
  (params (DeltaSeconds :type Float%20%28single-precision%29))
  (if (Math|Boolean|ORBoolean (Variables|Default|GetIsWatering?) (Variables|Default|GetPlanting?) (Variables|Default|GetIsRake))
    (Rendering|SetVisibility (Variables|Default|GetGrid) true false))
  (if (Variables|Default|GetIsWatering?)
    (Rendering|Material|CreateDynamicMaterialInstance (Variables|Default|GetGrid) 0 "/Game/Material/Tierra_Mojada.Tierra_Mojada" "None" :!class /Script/Engine.PrimitiveComponent)
    (elif (Variables|Default|GetIsRake)
      (Rendering|Material|CreateDynamicMaterialInstance (Variables|Default|GetGrid) 0 "/Game/Material/Tierra_arada.Tierra_arada" "None" :!class /Script/Engine.PrimitiveComponent)
      (else
        (Rendering|Material|CreateDynamicMaterialInstance (Variables|Default|GetGrid) 0 "/Game/Material/Tierra.Tierra" "None" :!class /Script/Engine.PrimitiveComponent)))))

(event Input|ActionEvents|InputActionInteract
  (params (Key :type Key%20Structure :default "None"))
  (:Pressed
    (CallFunction|Arrar?sembrar)))

(fn ConstructionScript)

(fn Arrar?sembrar
  (bind _self self)
  (bind _returnvalue (Transformation|GetActorLocation _self))
  (bind (_x _y) (Math|Vector|BreakVector _returnvalue))
  (bind _asplayer_character (Utilities|Casting|CastToPlayer_Character (Game|GetPlayerCharacter 0)))
  (switch Utilities|FlowControl|Switch|SwitchonType_Obj (.type_obj (Variables|/Game/Blueprints/Characters/Player_Character/Player_Character.Player_Character_C|GetType%20Obj%20Slot _asplayer_character))
    (:NewEnumerator0
      (if (Utilities|Enum|Equal(Enum) (.name (Variables|/Game/Blueprints/Characters/Player_Character/Player_Character.Player_Character_C|GetType%20Obj%20Slot _asplayer_character)) (Variables|Default|GetHoe))
        (if (not (Variables|Default|GetIsRake))
          (if (Variables|Default|GetIsWatering?)
            (Rendering|Material|CreateDynamicMaterialInstance (Variables|Default|GetGrid) 0 "/Game/Material/Tierra_Mojada.Tierra_Mojada" "None" :!class /Script/Engine.PrimitiveComponent)
            (else
              (Rendering|Material|CreateDynamicMaterialInstance (Variables|Default|GetGrid) 0 "/Game/Material/Tierra_arada.Tierra_arada" "None" :!class /Script/Engine.PrimitiveComponent)))
          (Rendering|SetVisibility (Variables|Default|GetGrid) true false)
          (Variables|Default|SetIsRake true))
        (elif (Utilities|Enum|Equal(Enum) (.name (Variables|/Game/Blueprints/Characters/Player_Character/Player_Character.Player_Character_C|GetType%20Obj%20Slot _asplayer_character)) (Variables|Default|GetWateringCan))
          (if (Variables|Default|GetIsRake)
            (if (not (Variables|Default|GetIsWatering?))
              (if (Variables|Default|GetPlanting?)
                (bind _asplayer_character_2 (Utilities|Casting|CastToPlayer_Character (Game|GetPlayerCharacter 0)))
                (if (> (Variables|/Game/Blueprints/Actors/Herramientas/WateringCan.WateringCan_C|GetWater (Variables|/Game/Blueprints/Widgets/Inventario/PlayerInventorySlot_UI.PlayerInventorySlot_UI_C|GetWatherinCan (Variables|/Game/Blueprints/Characters/Player_Character/Player_Character.Player_Character_C|GetMenuSlots_Use _asplayer_character_2))) 9)
                  (Variables|Default|SetIsWatering? true)
                  (Default|UsarHerramiento (Variables|/Game/Blueprints/Widgets/Inventario/PlayerInventorySlot_UI.PlayerInventorySlot_UI_C|GetWatherinCan (Variables|/Game/Blueprints/Characters/Player_Character/Player_Character.Player_Character_C|GetMenuSlots_Use _asplayer_character_2)))
                  (Variables|Default|SetCalidad_Cuido (+ (Variables|Default|GetCalidad_Cuido) 1))
                  (Rendering|Material|CreateDynamicMaterialInstance (Variables|Default|GetGrid) 0 "/Game/Material/Tierra_Mojada.Tierra_Mojada" "None" :!class /Script/Engine.PrimitiveComponent))))))))
    (:NewEnumerator2
      (if (Variables|Default|GetIsRake)
        (if (not (Variables|Default|GetPlanting?))
          (bind _returnvalue_2 (Utilities|GetDataTableRow "/Game/Blueprints/DataTables/DataTable_Items_-_Hoja_1.DataTable_Items_-_Hoja_1" (Utilities|String|StringToName (Utilities|String|ToString(Integer) (.id_reference (Variables|/Game/Blueprints/Characters/Player_Character/Player_Character.Player_Character_C|GetType%20Obj%20Slot _asplayer_character)))))
            (:then
              (bind _returnvalue_3 (Game|SpawnActorfromClass (.objeto _returnvalue_2) (Math|Transform|MakeTransform (Math|Vector|MakeVector _x _y 138.0)) "Undefined" 0 0))
              (Variables|Default|SetType_Plant _returnvalue_3)
              (Variables|Default|SetPlanting? true)
              (bind _asplayer_character_3 (Utilities|Casting|CastToPlayer_Character (Game|GetPlayerCharacter 0)))
              (Default|Eliminacion (Variables|/Game/Blueprints/Characters/Player_Character/Player_Character.Player_Character_C|GetMision_Component _asplayer_character_3) (.objeto _returnvalue_2))
              (bind _asplayer_character_4 (Utilities|Casting|CastToPlayer_Character (Game|GetPlayerCharacter 0)))
              (for _array_element (Variables|/Game/Blueprints/Characters/Player_Character/Player_Character.Player_Character_C|GetMenuSlots_Array _asplayer_character_4)
                (if (== (Variables|/Game/Blueprints/Widgets/Inventario/PlayerInventorySlot_UI.PlayerInventorySlot_UI_C|GetNum_Slot _array_element) (Variables|/Game/Blueprints/Characters/Player_Character/Player_Character.Player_Character_C|GetNum_Slot _asplayer_character_4))
                  (Default|RemovefromInventory (Variables|/Game/Blueprints/Characters/Player_Character/Player_Character.Player_Character_C|GetInventory_component _asplayer_character_4) (Variables|/Game/Blueprints/Widgets/Inventario/PlayerInventorySlot_UI.PlayerInventorySlot_UI_C|GetItem_ID _array_element)))))))))))

(fn SetGrid
  (Rendering|SetVisibility (Variables|Default|GetGrid) false false)
  (Rendering|Material|CreateDynamicMaterialInstance (Variables|Default|GetGrid) 0 "/Game/Material/Tierra.Tierra" "None" :!class /Script/Engine.PrimitiveComponent)
  (Variables|Default|SetCalidad_Cuido 0)
  (Variables|Default|SetIsWatering? false)
  (Variables|Default|SetPlanting? false)
  (Variables|Default|SetIsRake false))

(fn AumentarSiEstallovindo
  (if (Variables|Default|GetPlanting?)
    (Variables|Default|SetCalidad_Cuido (+ (Variables|Default|GetCalidad_Cuido) 1))))

(fn Iniciarsembrado
  (params (Planta :type Integer))
  (bind _self self)
  (bind _returnvalue (Transformation|GetActorLocation _self))
  (bind (_x _y) (Math|Vector|BreakVector _returnvalue))
  (Variables|Default|SetIsRake true)
  (if (Variables|Default|GetIsRake)
    (if (not (Variables|Default|GetPlanting?))
      (bind _returnvalue_2 (Utilities|GetDataTableRow "/Game/Blueprints/DataTables/DataTable_Items_-_Hoja_1.DataTable_Items_-_Hoja_1" (Utilities|String|StringToName (Utilities|String|ToString(Integer) Planta)))
        (:then
          (bind _returnvalue_3 (Game|SpawnActorfromClass (.objeto _returnvalue_2) (Math|Transform|MakeTransform (Math|Vector|MakeVector _x _y 138.0)) "Undefined" 0 0))
          (Variables|Default|SetType_Plant _returnvalue_3)
          (Variables|Default|SetPlanting? true))))))